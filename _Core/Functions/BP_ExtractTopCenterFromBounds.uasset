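; PCG Blueprint element that turns an attribute set's bounds into the location of the center of their top face.
; It reads BoundsMin and BoundsMax from the first entry of the first input param data, taking the X/Y midpoint and maximum Z.
; The result becomes the default value of a Location attribute on a new single-entry param data, returned as the output.
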(fn ExecutewithContext
  (params (InContext :type PCG%20Context%20Structure%20%28by%20ref%29) (Input :type PCG%20Data%20Collection%20Structure%20%28by%20ref%29))
  (bind _returnvalue (Data|GetParams Input))
  (bind _aspcgattribute_set (Utilities|Casting|CastToPCGParamData (.Data (PCG|TaggedData|BreakTaggedData (Utilities|Array|Get(acopy) _returnvalue)))))
  (bind _returnvalue_2 (Metadata|MutableMetadata _aspcgattribute_set))
  (bind _output_get (LocalVariables|SetInMetadata _returnvalue_2))
  (bind _returnvalue_3 (PCG|Metadata|GetVectorAttributebyMetadataKey 0 _output_get "BoundsMax"))
  (bind _returnvalue_4 (PCG|Metadata|GetVectorAttributebyMetadataKey 0 _output_get "BoundsMin"))
  (bind _returnvalue_5 (Game|ConstructObjectfromClass "/Script/PCG.PCGParamData"))
  (bind _returnvalue_6 (Metadata|MutableMetadata _returnvalue_5))
  (LocalVariables|SetOutMetadata _returnvalue_6)
  (PCG|Metadata|CreateVectorAttribute (LocalVariables|GetOutMetadata) "Location" (Math|Vector|MakeVector (+ (/ (- (.X (Math|Vector|BreakVector _returnvalue_3)) (.X (Math|Vector|BreakVector _returnvalue_4))) 2.0) (.X (Math|Vector|BreakVector _returnvalue_4))) (+ (.Y (Math|Vector|BreakVector _returnvalue_4)) (/ (- (.Y (Math|Vector|BreakVector _returnvalue_3)) (.Y (Math|Vector|BreakVector _returnvalue_4))) 2.0)) (.Z (Math|Vector|BreakVector _returnvalue_3))) false true)
  (PCG|Metadata|AddEntry (LocalVariables|GetOutMetadata) -1)
  (return (Utilities|Struct|MakePCGDataCollection (Utilities|Array|MakeArray (PCG|TaggedData|MakeTaggedData _returnvalue_5)))))