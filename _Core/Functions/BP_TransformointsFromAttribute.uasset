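; Custom PCG Blueprint node, titled TransformFromAttribute, that randomly shifts points horizontally using per-point attributes.
; Its point loop reads the OffsetMin and OffsetMax vectors and adds a random X and Y within that range to each location, leaving Z, rotation and scale unchanged.
; The offset uses plain RandomFloatInRange rather than a seeded random stream, so it is not tied to point seeds.
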(fn PointLoopBody
  (params (InContext :type PCG%20Context%20Structure%20%28by%20ref%29) (InData :type PCG%20Point%20Data%20Object%20Reference) (InPoint :type PCG%20Point%20Structure%20%28by%20ref%29) (OutMetadata :type PCG%20Metadata%20Object%20Reference) (Iteration :type Integer64))
  (bind _transform (Utilities|Struct|BreakPCGPoint InPoint))
  (bind _returnvalue (Metadata|ConstMetadata InData))
  (bind (_location _rotation _scale) (Math|Transform|BreakTransform _transform))
  (bind _returnvalue_2 (PCG|Metadata|GetVectorAttribute InPoint _returnvalue "OffsetMin"))
  (bind _returnvalue_3 (PCG|Metadata|GetVectorAttribute InPoint _returnvalue "OffsetMax"))
  (Utilities|Struct|SetmembersinPCGPoint InPoint (Math|Transform|MakeTransform (+ (Math|Vector|MakeVector (Math|Random|RandomFloatinRange (.X (Math|Vector|BreakVector _returnvalue_2)) (.X (Math|Vector|BreakVector _returnvalue_3))) (Math|Random|RandomFloatinRange (.Y (Math|Vector|BreakVector _returnvalue_2)) (.Y (Math|Vector|BreakVector _returnvalue_3))) 0.0) _location) _rotation _scale))
  (return "" true))

(fn NodeTitleOverride
  (return "TransformFromAttribute"))

(fn NodeColorOverride
  (return "(R=1.000000,G=0.179815,B=0.000000,A=1.000000)"))