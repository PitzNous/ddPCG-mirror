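; BP_ExtractPlantMeshes is a custom PCG node that turns a plant species name into a list of its static meshes.
; It reads the Name attribute from the first entry of the input param data and finds the matching species in BiomeData's GroundVegetation.
; It outputs new param data with one entry per mesh, storing each path in a StaticMesh soft object path attribute.
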(fn NodeTitleOverride
  (return "ExtractPlantMeshes"))

(fn ExecutewithContext
  (params (InContext :type PCG%20Context%20Structure%20%28by%20ref%29) (Input :type PCG%20Data%20Collection%20Structure%20%28by%20ref%29))
  (bind _returnvalue (Data|GetParams Input))
  (bind _aspcgattribute_set (Utilities|Casting|CastToPCGParamData (.Data (PCG|TaggedData|BreakTaggedData (Utilities|Array|Get(acopy) _returnvalue)))))
  (bind _returnvalue_2 (Metadata|MutableMetadata _aspcgattribute_set))
  (bind _output_get (Variables|Default|SetInMetadata _returnvalue_2))
  (bind _returnvalue_3 (PCG|Metadata|GetStringAttributebyMetadataKey 0 _output_get "Name"))
  (LocalVariables|SetSpeciesName _returnvalue_3)
  (bind _returnvalue_4 (Game|ConstructObjectfromClass "/Script/PCG.PCGParamData"))
  (bind _returnvalue_5 (Metadata|MutableMetadata _returnvalue_4))
  (LocalVariables|SetOutMetadata _returnvalue_5)
  (PCG|Metadata|CreateSoftObjectPathAttribute (LocalVariables|GetOutMetadata) "StaticMesh" (Class|KismetSystemLibrary|MakeSoftClassPath) false true)
  (for _array_element (Variables|/Game/pitzclifftool/Core/CoreAssets/PDA_BiomeV2.PDA_BiomeV2_C|GetGroundVegetation (Variables|Default|GetBiomeData))
    (if (Utilities|Enum|Equal(Enum) (.Name (Utilities|Struct|BreakS_Species _array_element)) (LocalVariables|GetSpeciesName))
      (for _array_element_2 (.Meshes (Utilities|Struct|BreakS_Species _array_element))
        (bind _returnvalue_6 (PCG|Metadata|AddEntry (LocalVariables|GetOutMetadata) -1))
        (Class|PCGMetadataAccessorHelpers|SetSoftObjectPathAttributebyMetadataKey _returnvalue_6 (LocalVariables|GetOutMetadata) "StaticMesh" (Utilities|GetSoftObjectPath (.StaticMesh (Utilities|Struct|BreakS_FallBack _array_element_2)))))
      (return (Utilities|Struct|MakePCGDataCollection (Utilities|Array|MakeArray (PCG|TaggedData|MakeTaggedData _returnvalue_4)))))))