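; BP_NormalFromRot is a PCG Blueprint node, titled "Normal From Rot", that derives a "Normal" vector attribute from point rotation.
; Its point loop body adds a metadata entry parented to each point's entry and writes roll, pitch and yaw there as raw XYZ, not a direction vector.
; The body passes the input point out without assigning it the new entry key, and returns false.
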(fn NodeTitleOverride
  (return "Normal From Rot"))

(fn NodeColorOverride
  (return "(R=0.000000,G=0.301660,B=1.000000,A=1.000000)"))

(fn PointLoopBody
  (params (InContext :type PCG%20Context%20Structure%20%28by%20ref%29) (InData :type PCG%20Point%20Data%20Object%20Reference) (InPoint :type PCG%20Point%20Structure%20%28by%20ref%29) (OutMetadata :type PCG%20Metadata%20Object%20Reference) (Iteration :type Integer64))
  (bind (_transform _density _boundsmin _boundsmax _color _steepness _seed _metadataentry) (Utilities|Struct|BreakPCGPoint InPoint))
  (bind _rotation (Math|Transform|BreakTransform _transform))
  (bind (_roll _pitch _yaw) (Math|Rotator|BreakRotator _rotation))
  (bind _returnvalue (PCG|Metadata|AddEntry OutMetadata _metadataentry))
  (PCG|Metadata|SetVectorAttributebyMetadataKey _returnvalue OutMetadata "Normal" (Math|Vector|MakeVector _roll _pitch _yaw))
  (return InPoint false))