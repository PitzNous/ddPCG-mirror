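; BP_PCGSetDressTool is a set dressing tool Blueprint that wraps a PCG component.
; Its Regenerate event assigns a random seed, cleans up the previous output and generates again, while Cleanup only clears the output.
; The construction script copies the component's graph instance into a GraphInstance variable.
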(event Custom|Cleanup
  (Class|PCGComponent|Cleanup (Variables|Default|GetPCG) true))

(event Custom|Regenerate
  (bind _pcg (Variables|Default|GetPCG))
  (Variables|/Script/PCG.PCGComponent|SetSeed _pcg (Math|Random|RandomInteger 999999999))
  (Class|PCGComponent|Cleanup _pcg true)
  (PCG|Generate _pcg true))

(event EventBeginPlay)

(event Collision|EventActorBeginOverlap
  (params (OtherActor :type Actor%20Object%20Reference)))

(event EventTick
  (params (DeltaSeconds :type Float%20%28single-precision%29)))

(fn ConstructionScript
  (Variables|Default|SetGraph%20Instance (Variables|/Script/PCG.PCGComponent|GetGraphInstance (Variables|Default|GetPCG))))