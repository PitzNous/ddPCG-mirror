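; A legacy foliage spawning volume actor that generates biome-specific foliage through a PCG component.
; BuildFoliage writes BiomeType into the PCG graph instance parameter and triggers local generation, while Cleanup clears the generated result.
; The construction script sizes the box from BoxExtent with extra vertical height, and KMS destroys the actor.
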(event Custom|KMS
  (Actor|DestroyActor))

(event Custom|BuildFoliage
  (Audio|Parameter|SetObjectParameter (Variables|/Script/PCG.PCGComponent|GetGraphInstance (Variables|Default|GetPCG)) "BiomeType" (.BiomeType (Variables|Default|GetBiomeType)))
  (PCG|Generate (Variables|Default|GetPCG) false))

(event Custom|Cleanup
  (Class|PCGComponent|Cleanup (Variables|Default|GetPCG) false))

(event EventBeginPlay)

(event Collision|EventActorBeginOverlap
  (params (OtherActor :type Actor%20Object%20Reference)))

(event EventTick
  (params (DeltaSeconds :type Float%20%28single-precision%29)))

(fn ConstructionScript
  (Components|Box|SetBoxExtent (Variables|Default|GetBox) (+ (Variables|Default|GetBoxExtent) "0.000000,0.000000,5000.000000") true))