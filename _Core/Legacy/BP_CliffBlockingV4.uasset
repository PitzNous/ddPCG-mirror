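; Legacy cliff blocking actor that uses PCG to generate rocks from a biome preset, unless flagged blocking-only.
; Construction and Build events reseed and generate the graph, while other events push size, density, offset and landscape-handling parameters.
; In foliage mode, PCG points become instances on InstancedFoliageActor HISMs, adding missing components and tracking instance IDs for removal.
; FinishJob increments a loop counter on the referenced UI to signal completion.
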(event OnPCGGraphGeneratedExternal(PCG)
  (params (PCGComponent :type PCG%20Component%20Object%20Reference))
  ;[1 1 1] FoliageConvertionSequence
  (if (Variables|Default|GetGenerateFoliageInstead)
    (CallFunction|PointtoFoliage)
    (CallFunction|AddFoliagetoCoordonate)
    (CallFunction|FinishJob)
    (else
      (CallFunction|FinishJob))))

(event Custom|Build
  (params (EUWRef :type %20Object%20Reference))
  (bind _pcg (Variables|Default|GetPCG))
  ;[1 1 1] GeneratePCG
  (if (Variables|Default|GetIsBlockingOnly)
    (CallFunction|FinishJob)
    (else
      (Variables|/Script/PCG.PCGComponent|SetSeed _pcg (Math|Conversions|ToInteger(Byte) (Class|KismetMathLibrary|RandomInteger64)))
      (PCG|Generate _pcg false)
      (CallFunction|FoliageGenerationSequence))))

(event Custom|Cleanup
  (params (EUWRef :type %20Object%20Reference))
  ;[1 1 1] CleanupPCG
  (Variables|Default|SetLastUsedUIRef 0 EUWRef)
  (Class|PCGComponent|Cleanup (Variables|Default|GetPCG) true)
  (CallFunction|ClearFoliage)
  (CallFunction|FinishJob))

(event Custom|FoliageGenerationSequence
  ;[1 1 1] FoliageConvertionSequence
  (if (Variables|Default|GetGenerateFoliageInstead)
    (CallFunction|PointtoFoliage)
    (CallFunction|AddFoliagetoCoordonate)
    (CallFunction|FinishJob)
    (else
      (CallFunction|FinishJob))))

(event Custom|NewValues
  (params (SizeMax :type Float%20%28double-precision%29) (SizeMin :type Float%20%28double-precision%29) (Density :type Float%20%28double-precision%29) (Offset :type Float%20%28double-precision%29) (EuwRef :type %20Object%20Reference))
  (bind _pcg (Variables|Default|GetPCG))
  (bind _graphinstance (Variables|/Script/PCG.PCGComponent|GetGraphInstance _pcg))
  ;[1 1 1] Update PCG Settings
  (Variables|Default|SetLastUsedUIRef 0 EuwRef)
  (Effects|Components|ParticleSystem|SetFloatParameter _graphinstance "Density" Density)
  (Effects|Components|ParticleSystem|SetFloatParameter _graphinstance "TopOffset" Offset)
  (Effects|Components|ParticleSystem|SetFloatParameter _graphinstance "SizeMax" SizeMax)
  (Effects|Components|ParticleSystem|SetFloatParameter _graphinstance "SizeMin" SizeMin)
  (CallFunction|SetMeshList)
  (CallFunction|FinishJob))

(event Custom|UpdateUseFoliagebool
  (params (NewValue :type Boolean))
  (bind _output_get (Variables|Default|SetGenerateFoliageInstead NewValue))
  (Effects|Components|ParticleSystem|SetBoolParameter (Variables|/Script/PCG.PCGComponent|GetGraphInstance (Variables|Default|GetPCG)) "GenerateFoliage" _output_get)
  (CallFunction|Build))

(event Collision|EventActorBeginOverlap
  (params (OtherActor :type Actor%20Object%20Reference)))

(event EventTick
  (params (DeltaSeconds :type Float%20%28single-precision%29))
  ;[1 1 1] GeneratePCG
)

(fn ConstructionScript
  (if (Variables|Default|GetIsBlockingOnly)
    (Utilities|Array|Clear (Variables|Actor|GetTags))
    (else
      (Variables|/Script/PCG.PCGComponent|SetSeed (Variables|Default|GetPCG) (Math|Random|RandomInteger 0))
      (CallFunction|SetMeshList)
      (CallFunction|Build))))

(fn SetMeshList
  (Audio|Parameter|SetObjectParameter (Variables|/Script/PCG.PCGComponent|GetGraphInstance (Variables|Default|GetPCG)) "RockMeshes" (.BiomePreset (Variables|Default|GetBiomePreset))))

(fn AddFoliagetoCoordonate
  (CallFunction|AddMissingFoliages)
  (CallFunction|ClearFoliage)
  (bind _outactors (Actor|GetAllActorsOfClass "/Script/Foliage.InstancedFoliageActor"))
  (for _array_element _outactors
    (for _array_element_2 (Actor|GetComponentsByClass _array_element "/Script/Engine.HierarchicalInstancedStaticMeshComponent")
      (for _array_element_3 0
        (if (== (.Mesh (Utilities|Struct|Break _array_element_3)) (Variables|/Script/Engine.StaticMeshComponent|GetStaticMesh _array_element_2))
          (bind _returnvalue (Components|InstancedStaticMesh|AddInstances _array_element_2 (.TransformList (Utilities|Struct|Break _array_element_3)) true false true))
          (Utilities|Array|AddUnique 0 (Utilities|Struct|Make _array_element_2 _returnvalue)))))))

(fn PointtoFoliage
  (CallFunction|InitCoordList)
  (for _array_element (.TaggedData (Utilities|Struct|BreakPCGDataCollection (Class|PCGComponent|GetGeneratedGraphOutput (Variables|Default|GetPCG))))
    (bind _aspcgpoint_data (Utilities|Casting|CastToPCGPointData (.Data (PCG|TaggedData|BreakTaggedData _array_element))))
    (for _array_element_2 (SpatialData|GetPoints _aspcgpoint_data)
      (bind _returnvalue (Class|PCGMetadataAccessorHelpers|GetSoftObjectPathAttribute _array_element_2 (Metadata|ConstMetadata _aspcgpoint_data) "FoliageMesh"))
      (bind _array_element_3 (Utilities|Array|ForEachLoopwithBreak (Variables|Default|GetCliffsRocks (.BiomePreset (Variables|Default|GetBiomePreset))))
        (:LoopBody
          (if (== (Utilities|ResolveSoftReference (.FoliageMesh (Utilities|Struct|Break _array_element_3))) (Class|KismetSystemLibrary|ToSoftObjRef(SoftObjPath) _returnvalue))
            (for (_array_element_4 _array_index) 0
              (if (== (.Mesh (Utilities|Struct|Break _array_element_4)) (.StaticMesh (Utilities|Struct|Break _array_element_3)))
                (bind _output_get (LocalVariables|SetTempTransArray (.TransformList (Utilities|Struct|Break _array_element_4))))
                (Utilities|Array|AddUnique _output_get (Utilities|Struct|BreakPCGPoint _array_element_2))
                (Utilities|Array|SetArrayElem 0 _array_index (Utilities|Struct|Make (.Mesh (Utilities|Struct|Break _array_element_4)) (LocalVariables|GetTempTransArray)))))))))))

(fn AddMissingFoliages
  ;[1 1 1] Check if any of the foliage instance component are from the foliage types of the biome, if not, create one
  (bind _outactors (Actor|GetAllActorsOfClass "/Script/Foliage.InstancedFoliageActor"))
  (for _array_element _outactors
    (bind _array_element_2 (Utilities|Array|ForEachLoopwithBreak (Variables|Default|GetCliffsRocks (.BiomePreset (Variables|Default|GetBiomePreset))))
      (:LoopBody
        (Variables|Default|SetFoliageAlreadyExist false)
        (for _array_element_3 (Actor|GetComponentsByClass _array_element "/Script/Engine.HierarchicalInstancedStaticMeshComponent")
          (if (== (Variables|/Script/Engine.StaticMeshComponent|GetStaticMesh _array_element_3) (Utilities|Struct|Break _array_element_2))
            (Variables|Default|SetFoliageAlreadyExist true)))
        (if (Variables|Default|GetFoliageAlreadyExist)
          (Variables|Default|SetFoliageAlreadyExist false)
          (else
            (bind _returnvalue (AddComponent|AddHierarchicalInstancedStaticMeshComponent _array_element false))
            (Components|StaticMesh|SetStaticMesh _returnvalue (Utilities|Struct|Break _array_element_2))
            (Development|PrintString (Utilities|GetDisplayName (Utilities|Struct|Break _array_element_2)))))))))

(fn InitCoordList
  (Utilities|Array|Clear 0)
  (for _array_element (Variables|Default|GetCliffsRocks (.BiomePreset (Variables|Default|GetBiomePreset)))
    (Utilities|Array|Add 0 (Utilities|Struct|Make (Utilities|Struct|Break _array_element)))))

(fn ClearFoliage
  (for _array_element 0
    (Class|InstancedStaticMeshComponent|RemoveInstances (.LinkedFoliageComponent (Utilities|Struct|Break _array_element)) (.Ids (Utilities|Struct|Break _array_element))))
  (Utilities|Array|Clear 0))

(fn FinishJob
  (bind _lastuseduiref (Variables|Default|GetLastUsedUIRef))
  (Variables|Default|SetCurrentLoopIteration _lastuseduiref (+ (Variables|Default|GetCurrentLoopIteration _lastuseduiref) 1.0)))

(fn ToggleLandscapeHandling
  (params (NewValue :type Boolean))
  (bind _output_get (Variables|Default|SetbLandscapeHandlingEnable? NewValue))
  (Effects|Components|ParticleSystem|SetBoolParameter (Variables|/Script/PCG.PCGComponent|GetGraphInstance (Variables|Default|GetPCG)) "UseLandscapeHandling" _output_get))